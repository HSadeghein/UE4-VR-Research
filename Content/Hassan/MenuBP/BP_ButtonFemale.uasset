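; BP_ButtonFemale is a pressable 3D menu button labeled "Female".
; Its construction script sets the label text, then runs the parent construction script.
; On Pressed, a timeline animates the button mesh's Z scale by an offset from its starting scale, with a flag blocking repeat presses until it finishes.
; The file contains only this press feedback, with no gender selection logic.
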(event EventBeginPlay
  (|CallParentFunction) ; This node is disabled and will not be called.\nDrag off pins to build functionality.
)

(event Collision|EventActorBeginOverlap
  (params (OtherActor :type Actor%20Object%20Reference))
  (|CallParentFunction OtherActor) ; This node is disabled and will not be called.\nDrag off pins to build functionality.
)

(event EventTick
  (params (DeltaSeconds :type Float%20%28single-precision%29))
  (|CallParentFunction DeltaSeconds) ; This node is disabled and will not be called.\nDrag off pins to build functionality.
)

(event EventPressed
  (if (not (Variables|Default|GetDisablePress))
    (Variables|Default|SetDisablePress true)
    (Variables|Default|SetInitialScale (Transformation|GetWorldScale (Variables|Default|Getbutton)))
    (bind _scale (Timeline|Scale PlayFromStart)
      (:Update
        (Transformation|SetWorldScale3D (Variables|Default|Getbutton) (Math|Vector|MakeVector (.X (Math|Vector|BreakVector (Variables|Default|GetInitialScale))) (.Y (Math|Vector|BreakVector (Variables|Default|GetInitialScale))) (+ (.Z (Math|Vector|BreakVector (Variables|Default|GetInitialScale))) (* _scale (Variables|Default|GetOffset))))))
      (:Finished
        (Variables|Default|SetDisablePress false)))))

(fn ConstructionScript
  (Variables|Default|SetButtonText "Female")
  (|CallParentFunction))