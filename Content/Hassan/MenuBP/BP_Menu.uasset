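; BP_Menu is a menu actor that presents Male and Female button actors, likely for a gender choice.
; On BeginPlay it spawns BP_ButtonMale and BP_ButtonFemale side by side, offset in world space from its Cube component and scaled down.
; Both buttons attach to the menu, keeping world location and scale while snapping rotation to it.
; It holds no selection logic itself.
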(event EventBeginPlay
  (bind _cube (Variables|Default|GetCube))
  (bind _returnvalue (Transformation|GetWorldLocation _cube))
  (bind _returnvalue_2 (- _returnvalue "5.000000,0.000000,0.000000"))
  (Utilities|FlowControl|Sequence
    (:then_0
      (bind _returnvalue_3 (Game|SpawnActorfromClass "/Game/Hassan/MenuBP/BP_ButtonMale.BP_ButtonMale_C" (Math|Transform|MakeTransform _returnvalue_2 "0, 0, 0" "0.050000,0.050000,0.020000") "Undefined" 0 0))
      (Transformation|AttachActorToActor _returnvalue_3 self "None" "KeepWorld" "SnapToTarget" "KeepWorld" true))
    (:then_1
      (bind _returnvalue_4 (Game|SpawnActorfromClass "/Game/Hassan/MenuBP/BP_ButtonFemale.BP_ButtonFemale_C" (Math|Transform|MakeTransform (+ _returnvalue_2 "12.000000,0.000000, 0") "0, 0, 0" "0.050000,0.050000,0.020000") "Undefined" 0 0))
      (Transformation|AttachActorToActor _returnvalue_4 self "None" "KeepWorld" "SnapToTarget" "KeepWorld" true))))

(event Collision|EventActorBeginOverlap
  (params (OtherActor :type Actor%20Object%20Reference)))

(event EventTick
  (params (DeltaSeconds :type Float%20%28single-precision%29)))

(fn ConstructionScript)