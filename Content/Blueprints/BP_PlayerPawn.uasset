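; VR player pawn that drives a full-body IK avatar with calibration, object grabbing and thumbstick sliding locomotion.
; VRIKBody feeds VRIKSkeletalMeshTranslator; calibration restores from a save game, or triggers reset and auto-calibrate it using a helper actor.
; Grips attach overlapping InteractiveActorInterface actors to avatar hand sockets and store their grab poses.
; While the right thumbstick is pressed, Tick slides the pawn horizontally relative to camera rotation, without sweep.
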(event Custom|RestoreCalibration
  (bind _calibrationhelper (Variables|Default|GetCalibrationHelper))
  ;[1 1 1] Load Calibration
  (Utilities|FlowControl|Delay 0.2)
  (bind (_bisvalid _calibrationdatavalue) (CallFunction|LoadCalibration))
  (if _bisvalid
    (Class|VRIKBody|RestoreCalibratedBody (Variables|Default|GetVRIKBody) _calibrationdatavalue)
    (Variables|Default|SetbShouldCalibrate false)
    (CallFunction|SaveCalibration (Class|VRIKBody|GetCalibratedBody (Variables|Default|GetVRIKBody)))
    (Utilities|IsValid _calibrationhelper
      (:Is%20Valid
        (Actor|DestroyActor _calibrationhelper)))))

(event Custom|Locomotion
  (params (DeltaTime :type Float%20%28single-precision%29))
  (bind _returnvalue (Class|Actor|GetInputAxisKeyValue))
  (bind _returnvalue_2 (Class|Actor|GetInputAxisKeyValue))
  (bind _vrcamera (Variables|Default|GetVRCamera))
  (bind _returnvalue_3 (Transformation|GetWorldRotation _vrcamera))
  (bind _returnvalue_4 (* _returnvalue_2 -1.0))
  (bind _returnvalue_5 (Math|Vector|MakeVector _returnvalue_4 _returnvalue 0.0))
  (bind _returnvalue_6 (Math|Vector|RotateVector _returnvalue_5 _returnvalue_3))
  ;[0 0 0] Artificial Sliding Locomotion
  (if (Variables|Default|GetbUseSlidingLocomotion)
    (Transformation|SetActorLocation (+ (Transformation|GetActorLocation) (* (Math|Vector|Normalize (Math|Vector|MakeVector (.x _returnvalue_6) (.y _returnvalue_6) 0.0)) (* DeltaTime (Variables|Default|GetSlidingSpeed)))) false false)))

(event EventBeginPlay
  ;[1 1 1] Initialization
  (Utilities|FlowControl|Delay 0.2)
  (Utilities|FlowControl|Sequence
    (:then_0
      (Class|HeadMountedDisplayFunctionLibrary|SetTrackingOrigin "Floor")
      (Class|VRIKBody|Initialize (Variables|Default|GetVRIKBody) (Variables|Default|GetVRCamera) (Variables|Default|GetMotionControllerRight) (Variables|Default|GetMotionControllerLeft))
      (Class|VRIKSkeletalMeshTranslator|Initialize (Variables|Default|GetVRIKSkeletalMeshTranslator) (Variables|Default|GetSM_Avatar) (Variables|Default|GetVRIKBody)))
    (:then_1
      (bind _outactors (Actor|GetAllActorsOfClass "/Game/Blueprints/BP_CalibrationHelper.BP_CalibrationHelper_C"))
      (if (> (Utilities|Array|Length _outactors) 0)
        (Variables|Default|SetCalibrationHelper (Utilities|Array|Get(acopy) _outactors))))
    (:then_2
      (CallFunction|RestoreCalibration))))

(event EventTick
  (params (DeltaSeconds :type Float%20%28single-precision%29))
  ;[1 1 1] Locomotion
  (CallFunction|Locomotion DeltaSeconds))

(event Input|KeyboardEvents|MotionControllerRightTrigger
  (params (Key :type Key%20Structure))
  (bind _calibrationhelper (Variables|Default|GetCalibrationHelper))
  (bind _calibrationhelper_2 (Variables|Default|GetCalibrationHelper))
  ;[1 1 1] Load Calibration
  (:Pressed
    (if (Variables|Default|GetbShouldCalibrate)
      (bind _returnvalue (Class|VRIKBody|AutoCalibrateBodyatPose (Variables|Default|GetVRIKBody)))
      (if _returnvalue
        (Variables|Default|SetbShouldCalibrate false)
        (CallFunction|SaveCalibration (Class|VRIKBody|GetCalibratedBody (Variables|Default|GetVRIKBody)))
        (Utilities|IsValid _calibrationhelper_2
          (:Is%20Valid
            (Actor|DestroyActor _calibrationhelper_2)))
        (else
          (Utilities|IsValid _calibrationhelper
            (:Is%20Valid
              (Default|TogglePose _calibrationhelper))))))))

(event Input|KeyboardEvents|MotionControllerRightGrip1
  (params (Key :type Key%20Structure))
  (:Pressed
    (CallFunction|TakeObject true))
  (:Released
    (CallFunction|ReleaseObject true)))

(event Input|KeyboardEvents|MotionControllerLeftGrip1
  (params (Key :type Key%20Structure))
  (:Pressed
    (CallFunction|TakeObject false))
  (:Released
    (CallFunction|ReleaseObject false)))

(event Input|KeyboardEvents|MotionControllerRightThumbstick
  (params (Key :type Key%20Structure))
  ;[1 1 1] Locomotion
  (:Pressed
    (Variables|Default|SetbUseSlidingLocomotion true))
  (:Released
    (Variables|Default|SetbUseSlidingLocomotion false)))

(event Input|KeyboardEvents|MotionControllerLeftTrigger
  (params (Key :type Key%20Structure))
  (bind _calibrationhelper (Variables|Default|GetCalibrationHelper))
  ;[1 1 1] Reset Calibration
  (:Pressed
    (Utilities|IsValid _calibrationhelper
      (:Is%20Valid
        (Rendering|SetActorHiddenInGame _calibrationhelper false)
        (Default|TogglePose _calibrationhelper)
        (Variables|Default|SetbShouldCalibrate true)
        (Class|VRIKBody|ResetCalibrationStatus (Variables|Default|GetVRIKBody))))))

(fn ConstructionScript)

(fn LoadCalibration
  (bind _returnvalue (SaveGame|CreateSaveGameObject "/Game/Blueprints/BP_SaveCalibration.BP_SaveCalibration_C"))
  (bind _returnvalue_2 (SaveGame|LoadGamefromSlot (Variables|/Game/Blueprints/BP_SaveCalibration.BP_SaveCalibration_C|GetFileName _returnvalue)))
  (bind _asbp_save_calibration (Utilities|Casting|CastToBP_SaveCalibration _returnvalue_2)
    (:then
      (return (Class|VRIKBody|IsValidCalibrationData (Variables|Default|GetVRIKBody) (Variables|/Game/Blueprints/BP_SaveCalibration.BP_SaveCalibration_C|GetCalibrationData _asbp_save_calibration)) (Variables|/Game/Blueprints/BP_SaveCalibration.BP_SaveCalibration_C|GetCalibrationData _asbp_save_calibration)))
    (:CastFailed
      (return false ""))))

(fn SaveCalibration
  (params (CalibrationData :type Calibrated%20Body%20Structure))
  (bind _returnvalue (SaveGame|CreateSaveGameObject "/Game/Blueprints/BP_SaveCalibration.BP_SaveCalibration_C"))
  (Variables|/Game/Blueprints/BP_SaveCalibration.BP_SaveCalibration_C|SetCalibrationData _returnvalue CalibrationData)
  (SaveGame|SaveGametoSlot _returnvalue (Variables|/Game/Blueprints/BP_SaveCalibration.BP_SaveCalibration_C|GetFileName _returnvalue)))

(fn TakeObject
  (params (bIsRightHand :type Boolean))
  (bind _array_element (Utilities|Array|ForEachLoopwithBreak (Collision|GetOverlappingActors (select bIsRightHand (Variables|Default|GetSphereR) (Variables|Default|GetSphereL)) "/Script/Engine.Actor" :!class /Script/Engine.PrimitiveComponent) :!label _label)
    (:LoopBody
      (if (Utilities|DoesObjectImplementInterface _array_element "/Game/Blueprints/InteractiveActorInterface.InteractiveActorInterface_C")
        (bind _returnvalue (Class|InteractiveActorInterface|CanGrab(Message) _array_element))
        (if _returnvalue
          (Utilities|FlowControl|Sequence
            (:then_0
              (Class|InteractiveActorInterface|Pickup(Message) _array_element (Variables|Default|GetSM_Avatar) (select bIsRightHand "hand_r" "hand_l") bIsRightHand)
              (bind _pose (Class|InteractiveActorInterface|GetGrabPose(Message) _array_element))
              (if bIsRightHand
                (Variables|Default|SetRightHandPose _pose)
                (Variables|Default|SetObjectInRightHand _array_element)
                (else
                  (Variables|Default|SetLeftHandPose _pose)
                  (Variables|Default|SetObjectInLeftHand _array_element))))
            (:then_1
              (goto _label Break))))))))

(fn ReleaseObject
  (params (bIsRightHand :type Boolean))
  (if bIsRightHand
    (Utilities|IsValid (Variables|Default|GetObjectInRightHand)
      (:Is%20Valid
        (Class|InteractiveActorInterface|Drop(Message) (Variables|Default|GetObjectInRightHand))
        (Variables|Default|SetObjectInRightHand 0)
        (Variables|Default|SetRightHandPose "NewEnumerator0")))
    (else
      (Utilities|IsValid (Variables|Default|GetObjectInLeftHand)
        (:Is%20Valid
          (Class|InteractiveActorInterface|Drop(Message) (Variables|Default|GetObjectInLeftHand))
          (Variables|Default|SetObjectInLeftHand 0)
          (Variables|Default|SetLeftHandPose "NewEnumerator0"))))))